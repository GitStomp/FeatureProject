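; AI controller for zombies that starts the BT_ZombieBehavior behavior tree on BeginPlay.
; Every Tick it polls AIPerception for player pawn 0 rather than binding to perception update events.
; It writes whether the first last-sensed stimulus was successful to the HasSeenPlayer Blackboard bool.
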(event `self.ReceiveBeginPlay`
  (`self.RunBehaviorTree` "/Game/Behavior/BT_ZombieBehavior.BT_ZombieBehavior"))

(event `self.ReceiveTick`
  (params (DeltaSeconds :type "Float (single-precision)"))
  (bind _returnvalue (`AIBlueprintHelperLibrary.GetBlackboard` (`AIBlueprintHelperLibrary.GetAIController` self)))
  (bind _info (`AIPerceptionComponent.GetActorsPerception` (`self.AIPerception`) (`GameplayStatics.GetPlayerPawn` 0)))
  (if (`.bSuccessfullySensed` (break `AIStimulus` (`|GetArrayItem` (`.LastSensedStimuli` (break `ActorPerceptionBlueprintInfo` _info)))))
    (`BlackboardComponent.SetValueAsBool` _returnvalue "HasSeenPlayer" true)
    (else
      (`BlackboardComponent.SetValueAsBool` _returnvalue "HasSeenPlayer" false))))

(fn `UserConstructionScript`)
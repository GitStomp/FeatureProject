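; BP_Zombie is an enemy that deals contact damage and destroys itself when its own health component reports death.
; On a hit, it damages any actor that has an AC_HealthComponent, so targets are not limited to the player.
; A LeaveAlone flag and a five-second delay act as an attack cooldown.
; BeginPlay caches a player pawn reference, which these graphs do not otherwise use.
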(event `self.ReceiveBeginPlay`
  ; get player reference
  (bind _asbp_player_pawn (cast `/Game/Blueprints/BP_PlayerPawn` (`GameplayStatics.GetPlayerPawn` 0)))
  (set `self.As BP Player Pawn` _asbp_player_pawn))

(event `self.AC_HealthComponent.OnDeath`
  ; destroy self on death
  (`self.K2_DestroyActor`))

(event `self.ReceiveHit`
  (params (MyComp :type "PrimitiveComponent Object Reference") (Other :type "Actor Object Reference") (OtherComp :type "PrimitiveComponent Object Reference") (bSelfMoved :type Boolean) (HitLocation :type "Vector Structure") (HitNormal :type "Vector Structure") (NormalImpulse :type "Vector Structure") (Hit :type "HitResult Structure (by ref)"))
  (bind _returnvalue (`self.GetComponentByClass` Other "/Game/Blueprints/AC_HealthComponent.AC_HealthComponent_C"))
  ; attack when in colliding
  (`/Engine/EditorBlueprintResources/StandardMacros.IsValid` _returnvalue
    (:`Is Valid`
      (if (not (`self.LeaveAlone`))
        (`/Game/Blueprints/AC_HealthComponent.TakeDamage` _returnvalue 1.0)
        (`KismetSystemLibrary.PrintString` "zombie hit")
        (set `self.LeaveAlone` true)
        (`KismetSystemLibrary.Delay` 5.0)
        (set `self.LeaveAlone` false)))))

(fn `UserConstructionScript`)